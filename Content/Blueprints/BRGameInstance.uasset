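; Game instance Blueprint that handles session matchmaking, joining an existing game or hosting a new one.
; TryJoinOrCreateGame destroys any current session, then searches over LAN or online via UseLAN, joining the first result through JoinBPSession.
; If the search fails or finds nothing, it creates a session and opens FirstPersonExampleMap as a listen server.
; Successful hosting or joining hides the cursor and sets game-only input, while create and join failures only print errors.
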(event Custom|Try%20Join%20Or%20Create%20Game
  (bind _returnvalue (Game|GetPlayerController 0))
  (bind _returnvalue_2 (Game|GetPlayerController 0))
  ;[1 1 1] Try Join, otherwise creates a session
  (|DestroySession _returnvalue
    (:OnSuccess
      _)
    (:OnFailure
      _))
  (bind _results (|FindSessions _returnvalue 20 (Variables|Default|GetUse%20LAN?))
    (:OnSuccess
      (if (Utilities|Array|IsValidIndex _results)
        (CallFunction|JoinBPSession (Utilities|Array|Get(acopy) _results))
        (else
          (|Session (Game|GetPlayerController 0) 20 (Variables|Default|GetUse%20LAN?) :!label _label
            (:OnSuccess
              (Game|OpenLevel(byName) "FirstPersonExampleMap" true "listen")
              (Variables|/Script/Engine.PlayerController|SetbShowMouseCursor _returnvalue_2 false)
              (Input|SetInputModeGameOnly _returnvalue_2))
            (:OnFailure
              (Development|PrintString "ERROR CREATING SESSION" true true "(R=1.000000,G=0.027276,B=0.000000,A=1.000000)" 5.0))))))
    (:OnFailure
      (goto _label))))

(event Custom|Join%20BP%20Session
  (params (Session :type Blueprint%20Session%20Result%20Structure))
  (bind _returnvalue (Game|GetPlayerController 0))
  ;[1 1 1] Join a session
  (|JoinSession (Game|GetPlayerController 0) Session
    (:OnSuccess
      (Variables|/Script/Engine.PlayerController|SetbShowMouseCursor _returnvalue false)
      (Input|SetInputModeGameOnly _returnvalue))
    (:OnFailure
      (Development|PrintString "ERROR JOINING SESSION" true true "(R=1.000000,G=0.027276,B=0.000000,A=1.000000)" 5.0))))