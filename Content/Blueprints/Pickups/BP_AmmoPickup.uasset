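; BP_AmmoPickup is a pickup actor that gives ammo to the weapon of a character who enters its sphere.
; On the PickupSphereEntered event, only the authority checks for a valid weapon, calls GiveAmmo with AmmoToGive, then destroys the pickup.
; A character without a valid weapon leaves the pickup in place.
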(event EventBeginPlay
  (|CallParentFunction) ; This node is disabled and will not be called.\nDrag off pins to build functionality.
)

(event Collision|EventActorBeginOverlap
  (params (OtherActor :type Actor%20Object%20Reference))
  (|CallParentFunction OtherActor) ; This node is disabled and will not be called.\nDrag off pins to build functionality.
)

(event EventTick
  (params (DeltaSeconds :type Float%20%28single-precision%29))
  (|CallParentFunction DeltaSeconds) ; This node is disabled and will not be called.\nDrag off pins to build functionality.
)

(event EventPickupSphereEntered
  (params (Character :type BR%20Character%20Object%20Reference))
  (bind _weapon (Variables|/Game/FirstPersonBP/Blueprints/BRCharacter.BRCharacter_C|GetWeapon Character))
  (Networking|SwitchHasAuthority
    (:Authority
      (Utilities|IsValid _weapon
        (:Is%20Valid
          (Default|GiveAmmo _weapon (Variables|Default|GetAmmoToGive))
          (Actor|DestroyActor))))))

(fn ConstructionScript
  (|CallParentFunction))