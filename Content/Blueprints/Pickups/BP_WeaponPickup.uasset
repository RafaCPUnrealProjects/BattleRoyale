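; BP_WeaponPickup is a weapon pickup that carries the clip and spare ammo for its WeaponToGive class.
; On BeginPlay, the server fills ammo from that class's defaults and calls parent BeginPlay only when DroppedByPlayer is false, so dropped weapons keep their ammo.
; Pickup sphere events set the character's CurrentWeaponPickup on entry and clear it on exit if it still references this pickup.
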(event EventBeginPlay
  (bind _weapontogive (Variables|Default|GetWeaponToGive))
  (bind (_damage _weaponname _currentammo _currentspareammo) (Utilities|GetClassDefaults _weapontogive))
  ;[1 1 1] Remember ammo amount if player drops the weapon
  (Networking|SwitchHasAuthority
    (:Authority
      (if (not (Variables|Default|GetDroppedByPlayer?))
        (Variables|Default|SetCurrentAmmoInClip _currentammo)
        (Variables|Default|SetCurrentSpareAmmo _currentspareammo)
        (|CallParentFunction)))))

(event Collision|EventActorBeginOverlap
  (params (OtherActor :type Actor%20Object%20Reference))
  (|CallParentFunction OtherActor) ; This node is disabled and will not be called.\nDrag off pins to build functionality.
)

(event EventTick
  (params (DeltaSeconds :type Float%20%28single-precision%29))
  (|CallParentFunction DeltaSeconds) ; This node is disabled and will not be called.\nDrag off pins to build functionality.
)

(event EventPickupSphereEntered
  (params (Character :type BR%20Character%20Object%20Reference))
  ;[1 1 1] Set player pickup
  (Variables|/Game/FirstPersonBP/Blueprints/BRCharacter.BRCharacter_C|SetCurrentWeaponPickup Character self))

(event EventPickupSphereLeft
  (params (Character :type BR%20Character%20Object%20Reference))
  ;[1 1 1] Unset player pickup
  (if (== (Variables|/Game/FirstPersonBP/Blueprints/BRCharacter.BRCharacter_C|GetCurrentWeaponPickup Character) self)
    (Variables|/Game/FirstPersonBP/Blueprints/BRCharacter.BRCharacter_C|SetCurrentWeaponPickup Character 0)))

(fn ConstructionScript
  (|CallParentFunction))